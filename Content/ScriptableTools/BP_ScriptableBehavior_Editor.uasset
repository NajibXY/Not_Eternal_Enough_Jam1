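; Scriptable editor tool for placing Light or Shadow level cubes on a grid in the viewport.
; A P_SnapProperty settings panel supplies cube type and grid size; hover line traces move a preview cube using M_HoverCube, cleared every second by a timer.
; Click spawns the mapped class unless the preview overlaps actors, while Shift-click destroys the hit actor.
; Setup snaps the viewport to a level camera, though only the Light branch returns a real transform.
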(event Custom|Clear%20each%201s%20the%20hover%20cube
  (HoverFunctions|ClearHoverCube))

(event EventOnScriptSetup
  (bind (_camera_location _camera_rotation) (CallFunction|ChooseWhichCameratoFindinScene))
  (CallFunction|SnapLevelViewportCameratoCamera _camera_location _camera_rotation)
  ;[0.15 0.15 0.15 0.5] Ajout des Properties dans la fenêtre a gauche du tool
  (bind _returnvalue (Class|ScriptableInteractiveTool|AddPropertySetOfType "/Game/ScriptableTools/P_SnapProperty.P_SnapProperty_C" "Settings")
    (:Success
      (bind _asp_snap_property (Utilities|Casting|CastToP_SnapProperty _returnvalue))
      (Variables|Default|SetAs%20P%20Snap%20Property _asp_snap_property)
      ;[0.15 0.15 0.15 0.5] Events on hover
      (Class|ScriptableModularBehaviorTool|AddMouseHoverBehavior (EventDispatchers|CreateEvent :!event BeginonHover) 0 (EventDispatchers|CreateEvent :!event UpdateonHover))
      (Utilities|Time|SetTimerbyEvent (delegate Custom|Clear%20each%201s%20the%20hover%20cube) 1.0 true)
      ;[0.15 0.15 0.15 0.5] Events on single click
      (Class|ScriptableModularBehaviorTool|AddSingleClickBehavior (EventDispatchers|CreateEvent :!event IfHitbyClick) (EventDispatchers|CreateEvent :!event OnHitbyClick)))))

(event EventOnScriptShutdown
  (params (ShutdownType :type EToolShutdownType%20Enum :default "Completed"))
  (HoverFunctions|ClearHoverCube))

(fn GetDatafromLineTraceHit
  (params (ClickPos :type Input%20Device%20Ray%20Structure))
  (bind (_startpoint _endpoint) (Class|GeometryScriptLibraryRayFunctions|GetRayStartEnd (.worldray ClickPos) 0.0 0.0))
  (bind _outhit (Collision|LineTraceByChannel _startpoint _endpoint "TraceTypeQuery1" false 0 "ForOneFrame"))
  (return (Class|ScriptableToolsUtilityLibrary|MakeInputRayHit (.distance _outhit)) (.distance _outhit) (.location _outhit) (.hitactor _outhit)))

(fn IfHitbyClick
  (params (ClickPos :type Input%20Device%20Ray%20Structure) (MouseButton :type EScriptableToolMouseButton%20Enum :default "LeftButton"))
  (bind _out_hit_distance (CallFunction|GetDatafromLineTraceHit ClickPos))
  (return (Class|ScriptableToolsUtilityLibrary|MakeInputRayHit _out_hit_distance)))

(fn OnHitbyClick
  (params (ClickPos :type Input%20Device%20Ray%20Structure) (Modifiers :type Scriptable%20Tool%20Modifier%20States%20Structure) (MouseButton :type EScriptableToolMouseButton%20Enum :default "LeftButton"))
  (if (Class|KismetInputLibrary|ModifierKeysStateIsShiftDown (Class|KismetInputLibrary|GetModifierKeysState))
    (bind _out_hit_actor (CallFunction|GetDatafromLineTraceHit ClickPos))
    (Utilities|IsValid _out_hit_actor
      (:Is%20Valid
        (Actor|DestroyActor _out_hit_actor))
      (:Is%20Not%20Valid
        (Development|PrintString "No object here")))
    (else
      (bind _out_hit_location (CallFunction|GetDatafromLineTraceHit ClickPos))
      (if (== (Utilities|Array|Length (Collision|GetOverlappingActors (Variables|Default|GetHover%20cube) 0 :!class /Script/Engine.Actor)) 0)
        (Game|SpawnActorfromClass (Parameters|GetActorClassfromSpawnMap) (Math|Transform|MakeTransform (Class|KismetMathLibrary|VectorSnappedtoGrid _out_hit_location (Variables|/Game/ScriptableTools/P_SnapProperty.P_SnapProperty_C|GetGridSize (Variables|Default|GetAs%20P%20Snap%20Property))) "0, 0, 0" "1.000000,1.000000,1.000000") "Undefined" "MultiplyWithRoot" 0 0)
        (else
          (Class|ScriptableInteractiveTool|DisplayUserWarningMessage "Alerte rouge Overlap"))))))

(fn BeginonHover
  (params (CurrentPos :type Input%20Device%20Ray%20Structure) (Modifiers :type Scriptable%20Tool%20Modifier%20States%20Structure))
  (bind (_startpoint _endpoint) (Class|GeometryScriptLibraryRayFunctions|GetRayStartEnd (.worldray CurrentPos) 0.0 0.0))
  (bind _outhit (Class|KismetSystemLibrary|LineTraceSinglebyProfile _startpoint _endpoint "None" false 0 "None" true))
  (return (Class|ScriptableToolsUtilityLibrary|MakeInputRayHit (.distance _outhit))))

(fn UpdateonHover
  (params (CurrentPos :type Input%20Device%20Ray%20Structure) (Modifiers :type Scriptable%20Tool%20Modifier%20States%20Structure))
  (bind _out_hit_location (CallFunction|GetDatafromLineTraceHit CurrentPos))
  (HoverFunctions|HoverCube _out_hit_location (Variables|Default|GetHover%20cube))
  (return false))

(fn HoverCube
  (params (Location :type Vector) (Hover%20cube :type Actor%20Object%20Reference))
  (bind _as_p_snap_property (Variables|Default|GetAs%20P%20Snap%20Property))
  (bind _gridsize (Variables|/Game/ScriptableTools/P_SnapProperty.P_SnapProperty_C|GetGridSize _as_p_snap_property))
  (bind _returnvalue (Class|KismetMathLibrary|VectorSnappedtoGrid Location _gridsize))
  (Utilities|IsValid Hover%20cube
    (:Is%20Valid
      (Transformation|SetActorTransform (Variables|Default|GetHover%20cube) (Math|Transform|MakeTransform _returnvalue "0, 0, 0" "1.000000,1.000000,1.000000")))
    (:Is%20Not%20Valid
      (bind _returnvalue_2 (Game|SpawnActorfromClass (Parameters|GetActorClassfromSpawnMap) (Math|Transform|MakeTransform _returnvalue "0, 0, 0" "1.000000,1.000000,1.000000") "Undefined" "MultiplyWithRoot" 0 0))
      (Variables|Default|SetHover%20cube _returnvalue_2)
      (|ChangeHoverCubematerial))))

(fn ClearHoverCube
  (Actor|DestroyActor (Variables|Default|GetHover%20cube)))

(fn GetActorClassfromSpawnMap
  (return (.Value (Utilities|Map|Find (Variables|Default|GetSpawnMap) (Parameters|GetObjecttoSpawnfromSnapProperty)))))

(fn GetObjecttoSpawnfromSnapProperty
  (return (Variables|/Game/ScriptableTools/P_SnapProperty.P_SnapProperty_C|GetObject%20to%20Spawn (Variables|Default|GetAs%20P%20Snap%20Property))))

(fn ChooseWhichCameratoFindinScene
  (bind _object_to_spawn (Parameters|GetObjecttoSpawnfromSnapProperty))
  (switch Utilities|FlowControl|Switch|SwitchonE_SpawnObject _object_to_spawn
    (:NewEnumerator0
      (bind _returnvalue (Actor|GetActorOfClass "/Game/BlueprintBlocks/BP_Camera_Light.BP_Camera_Light_C")))
    (:NewEnumerator1
      (Actor|GetActorOfClass "/Game/BlueprintBlocks/BP_Camera_Shadow.BP_Camera_Shadow_C")))
  (return (Utilities|Select :Index _object_to_spawn :NewEnumerator0 (Transformation|GetActorLocation _returnvalue) :NewEnumerator1 "0, 0, 0") (Utilities|Select :Index _object_to_spawn :NewEnumerator0 (Transformation|GetActorRotation _returnvalue) :NewEnumerator1 "0, 0, 0")))