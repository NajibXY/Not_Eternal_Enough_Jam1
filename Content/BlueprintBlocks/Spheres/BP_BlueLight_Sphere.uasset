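; BP_BlueLight_Sphere is a blue light sphere that publishes its position and size to the MPC_Blue material parameter collection.
; On BeginPlay it takes its index among all blue light spheres and writes its mesh location and X scale to the matching location and radius slot.
; Only the first three spheres get a slot.
; Tick refreshes those parameters while the sphere is following the mouse.
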(event EventBeginPlay
  (|CallParentFunction)
  (bind _outactors (Actor|GetAllActorsOfClass "BP_BlueLight_Sphere_C"))
  (for (_array_element _array_index) _outactors
    (if (== _array_element self)
      (Variables|Default|SetIndexOfBlue _array_index)))
  (Utilities|MakeBlueVisible))

(event EventTick
  (params (DeltaSeconds :type Float%20%28single-precision%29))
  (|CallParentFunction DeltaSeconds)
  (if (Variables|Default|GetIsFollowingMouse)
    (Utilities|MakeBlueVisible)))

(fn ConstructionScript
  (|CallParentFunction))