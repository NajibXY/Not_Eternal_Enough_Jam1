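; Light sphere for a side-scroller that makes BP_Cube_NANA_test cubes solid while they overlap it.
; Overlap begin sets the cube's mesh and box to BlockAll and overlap end to NoCollision, skipping the player character and shadow spheres, with debug prints.
; While IsFollowingMouse is set, Tick moves the sphere's mesh toward the cursor trace hit in X and Z, keeping Y, using the world hit as relative location.
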(event EventBeginPlay)

(event Collision|EventActorBeginOverlap
  (params (OtherActor :type Actor%20Object%20Reference))
  (Utilities|Casting|CastToBP_SideScrollerCharacter OtherActor
    (:CastFailed
      (Utilities|Casting|CastToBP_Shadow_Sphere OtherActor
        (:CastFailed
          (bind _asbp_cube_nana_test (Utilities|Casting|CastToBP_Cube_NANA_test OtherActor))
          (Development|PrintText "In")
          (Collision|SetCollisionProfileName (Variables|/Script/Engine.StaticMeshActor|GetStaticMeshComponent _asbp_cube_nana_test) "BlockAll" true :!class /Script/Engine.PrimitiveComponent)
          (Collision|SetCollisionProfileName (Variables|/Script/Engine.StaticMeshActor|GetStaticMeshComponent _asbp_cube_nana_test) "BlockAll" true :!class /Script/Engine.PrimitiveComponent)
          (Collision|SetCollisionProfileName (Variables|/Game/BlueprintBlocks/BP_Cube_NANA_test.BP_Cube_NANA_test_C|GetBox _asbp_cube_nana_test) "BlockAll" true :!class /Script/Engine.PrimitiveComponent))))))

(event EventTick
  (params (DeltaSeconds :type Float%20%28single-precision%29))
  (bind _returnvalue (Game|GetPlayerController 0))
  (bind _staticmeshcomponent (Variables|Debug|GetStaticMeshComponent))
  (bind _hitresult (Game|Player|GetHitResultUnderCursorbyChannel _returnvalue "TraceTypeQuery1" true))
  ;[0.15 0.15 0.15 0.5] Mouse logic
  (if (Variables|Default|GetIsFollowingMouse)
    (Components|MoveComponentTo _staticmeshcomponent (Math|Vector|MakeVector (.x (.location _hitresult)) (.y (Variables|/Script/Engine.SceneComponent|GetRelativeLocation _staticmeshcomponent)) (.z (.location _hitresult))) "0, 0, 0" false false 0.01 false)))

(event Collision|EventActorEndOverlap
  (params (OtherActor :type Actor%20Object%20Reference))
  (Utilities|Casting|CastToBP_SideScrollerCharacter OtherActor
    (:CastFailed
      (Utilities|Casting|CastToBP_Shadow_Sphere OtherActor
        (:CastFailed
          (bind _asbp_cube_nana_test (Utilities|Casting|CastToBP_Cube_NANA_test OtherActor))
          (Development|PrintText "Out")
          (Collision|SetCollisionProfileName (Variables|/Script/Engine.StaticMeshActor|GetStaticMeshComponent _asbp_cube_nana_test) "NoCollision" true :!class /Script/Engine.PrimitiveComponent)
          (Collision|SetCollisionProfileName (Variables|/Script/Engine.StaticMeshActor|GetStaticMeshComponent _asbp_cube_nana_test) "NoCollision" true :!class /Script/Engine.PrimitiveComponent)
          (Collision|SetCollisionProfileName (Variables|/Game/BlueprintBlocks/BP_Cube_NANA_test.BP_Cube_NANA_test_C|GetBox _asbp_cube_nana_test) "NoCollision" true :!class /Script/Engine.PrimitiveComponent))))))

(fn ConstructionScript)