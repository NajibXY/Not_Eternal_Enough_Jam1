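; BP_LightLevel_BaseCube is a light-level block that pawns can pass through while it overlaps a shadow sphere.
; When an actor of exact class BP_Shadow_Sphere begins overlapping, the static mesh's Pawn channel response switches to Ignore.
; When one stops overlapping, the response returns to Block, with no count of other spheres still overlapping.
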(event Collision|EventActorBeginOverlap
  (params (OtherActor :type Actor%20Object%20Reference))
  (if (== (Utilities|GetClass OtherActor) "/Game/BlueprintBlocks/BP_Shadow_Sphere.BP_Shadow_Sphere_C")
    (Collision|SetCollisionResponsetoChannel (Variables|Debug|GetStaticMeshComponent) "ECC_Pawn" "ECR_Ignore")))

(event Collision|EventActorEndOverlap
  (params (OtherActor :type Actor%20Object%20Reference))
  (if (== (Utilities|GetClass OtherActor) "/Game/BlueprintBlocks/BP_Shadow_Sphere.BP_Shadow_Sphere_C")
    (Collision|SetCollisionResponsetoChannel (Variables|Debug|GetStaticMeshComponent) "ECC_Pawn" "ECR_Block")))

(fn ConstructionScript)