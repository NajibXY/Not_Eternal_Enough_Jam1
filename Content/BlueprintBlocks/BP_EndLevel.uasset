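; BP_EndLevel is an end-of-level trigger that opens the editable next level when a pawn overlaps it.
; It prints a reminder if no next level name is set on the instance.
; Before loading, it copies the elapsed time from GM_SideScroller into BP_GameInstance.
; An editable IsLastLevel flag, meant for returns to chapter selection, turns the game instance's timer off; otherwise the timer is set active.
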(event EventBeginPlay)

(event Collision|EventActorBeginOverlap
  (params (OtherActor :type Actor%20Object%20Reference))
  ;[0.15 0.15 0.15 0.5] Mettre le nom du prochain niveau dans l'instance situé in game de ce blueprint
  (Utilities|Casting|CastToPawn OtherActor)
  (if (== (Variables|Default|GetNextLevel) (Variables|Default|GetNoneref))
    (Development|PrintString "Mettez le nom du prochain niveau dans l'instance de ce blueprint")
    (else
      ;[0.15 0.15 0.15 0.5] Variable éditable, à changer lors d'un retour en sélection chapitres
      (if (Variables|Default|GetIsLastLevel)
        ;[0.15 0.15 0.15 0.5] Désactive le timer et récupère le temps écoulé dans la game instance
        (bind _asgm_side_scroller (Utilities|Casting|CastToGM_SideScroller (Game|GetGameMode)))
        (bind _asbp_game_instance (Utilities|Casting|CastToBP_GameInstance (Game|GetGameInstance)))
        (Variables|/Game/Levels/BP_GameInstance.BP_GameInstance_C|SetTime _asbp_game_instance (Variables|/Game/Player/Blueprints/GM_SideScroller.GM_SideScroller_C|GetTime _asgm_side_scroller))
        (Variables|/Game/Levels/BP_GameInstance.BP_GameInstance_C|SetTimerActivated _asbp_game_instance false)
        (else
          ;[0.15 0.15 0.15 0.5] Récupère le temps écoulé et le stocke dans la game instance, et active le timer
          (bind _asgm_side_scroller_2 (Utilities|Casting|CastToGM_SideScroller (Game|GetGameMode)))
          (bind _asbp_game_instance_2 (Utilities|Casting|CastToBP_GameInstance (Game|GetGameInstance)))
          (Variables|/Game/Levels/BP_GameInstance.BP_GameInstance_C|SetTime _asbp_game_instance_2 (Variables|/Game/Player/Blueprints/GM_SideScroller.GM_SideScroller_C|GetTime _asgm_side_scroller_2))
          (Variables|/Game/Levels/BP_GameInstance.BP_GameInstance_C|SetTimerActivated _asbp_game_instance_2 true)))
      (Game|OpenLevel(byName) (Variables|Default|GetNextLevel)))))

(fn ConstructionScript)