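; Moving projectile that restarts the level on hitting a pawn, with lethality depending on light and shadow.
; BeginPlay treats levels without light spheres as lit, otherwise dark, and overlap counters on light and shadow spheres toggle the capsule's Pawn collision.
; ProjectileIsLight enables custom-depth stencil rendering and skips later overlap toggling.
; Tick offsets it along Direction, destroying it out of bounds; other overlaps set a speed-scaled lifespan.
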(event Custom|ProjectileIsLight
  (bind _sphere (Variables|Default|GetSphere))
  ;[0.15 0.15 0.15 0.5] If the Projectile appears in Shadow and can kill the player
  (Variables|Default|SetProjIsLight true)
  (Rendering|SetRenderCustomDepth _sphere true)
  (Rendering|SetCustomDepthStencilValue _sphere 1))

(event Collision|EventActorBeginOverlap
  (params (OtherActor :type Actor%20Object%20Reference))
  (bind _projislight (Variables|Default|GetProjIsLight))
  (bind _capsule (Variables|Collision|GetCapsule))
  (bind _lightcollisions (Variables|Default|GetLightCollisions))
  ;[0.15 0.15 0.15 0.5] Enter Shadow Sphere or Static light
  (Utilities|Casting|CastToBP_Shadow_Sphere OtherActor
    (:then
      (if (not _projislight)
        (Math|Integer|IncrementInt (Variables|Default|GetShadowCollisions)
          (:%20%20
            (if (== _lightcollisions 0)
              (Collision|SetCollisionResponsetoChannel _capsule "ECC_Pawn" "ECR_Ignore"))))))
    (:CastFailed
      (Utilities|Casting|CastToBP_Light_Sphere OtherActor
        (:then
          (if (not _projislight)
            (Math|Integer|IncrementInt _lightcollisions
              (:%20%20
                (Collision|SetCollisionResponsetoChannel _capsule "ECC_Pawn" "ECR_Overlap")))))
        (:CastFailed
          ;[0.15 0.15 0.15 0.5] Restart on hit
          (Utilities|Casting|CastToPawn OtherActor
            (:then
              (Utilities|FlowControl|Delay 0.1)
              (Development|ExecuteConsoleCommand "Restartlevel" 0))
            (:CastFailed
              ;[0.15 0.15 0.15 0.5] Destroy against Walls
              (Actor|SetLifeSpan (/ 0.1 (Variables|Default|Getspeed))))))))))

(event EventBeginPlay
  ;[0.15 0.15 0.15 0.5] Detect the type of the level and adapt its collisions
  (bind _outactors (Actor|GetAllActorsOfClass "/Game/BlueprintBlocks/Spheres/BP_Light_Sphere.BP_Light_Sphere_C"))
  (if (== (Utilities|Array|Length _outactors) 0)
    (Variables|Default|SetLightLevel true)
    (for _array_element (Collision|GetOverlappingActors "/Game/BlueprintBlocks/Spheres/BP_Shadow_Sphere.BP_Shadow_Sphere_C" :!class /Script/Engine.Actor)
      (Math|Integer|IncrementInt (Variables|Default|GetShadowCollisions)))
    (else
      (Variables|Default|SetLightLevel false)
      (Collision|SetCollisionResponsetoChannel (Variables|Collision|GetCapsule) "ECC_Pawn" "ECR_Ignore")
      (for _array_element_2 (Collision|GetOverlappingActors "/Game/BlueprintBlocks/Spheres/BP_Light_Sphere.BP_Light_Sphere_C" :!class /Script/Engine.Actor)
        (Math|Integer|IncrementInt (Variables|Default|GetLightCollisions))))))

(event EventTick
  (params (DeltaSeconds :type Float%20%28single-precision%29))
  (bind _returnvalue (Transformation|GetActorLocation))
  ;[0.15 0.15 0.15 0.5] Movement
  (if (or (or (< (.x _returnvalue) -3e+03) (> (.x _returnvalue) 3.5e+03)) (or (< (.z _returnvalue) -3.5e+03) (> (.z _returnvalue) 3e+03)))
    ;;[0.15 0.15 0.15 0.5] Destroy out of screen
    (Actor|DestroyActor)
    (else
      (Transformation|AddActorLocalOffset (* DeltaSeconds (* (Variables|Default|Getdirection) (Variables|Default|Getspeed))) false false))))

(event Collision|EventActorEndOverlap
  (params (OtherActor :type Actor%20Object%20Reference))
  (bind _lightlevel (Variables|Default|GetLightLevel))
  (bind _capsule (Variables|Collision|GetCapsule))
  ;[0.15 0.15 0.15 0.5] Exit Shadow Sphere or Static Light
  (if (not (Variables|Default|GetProjIsLight))
    (Utilities|Casting|CastToBP_Shadow_Sphere OtherActor
      (:then
        (bind _result (Math|Integer|DecrementInt (Variables|Default|GetShadowCollisions))
          (:%20%20
            (if (== _result 0)
              (if _lightlevel
                (Collision|SetCollisionResponsetoChannel _capsule "ECC_Pawn" "ECR_Overlap"))))))
      (:CastFailed
        (Utilities|Casting|CastToBP_Light_Sphere OtherActor)
        (bind _result_2 (Math|Integer|DecrementInt (Variables|Default|GetLightCollisions))
          (:%20%20
            (if (== _result_2 0)
              (if (not _lightlevel)
                (Collision|SetCollisionResponsetoChannel _capsule "ECC_Pawn" "ECR_Ignore")))))))))

(fn ConstructionScript)