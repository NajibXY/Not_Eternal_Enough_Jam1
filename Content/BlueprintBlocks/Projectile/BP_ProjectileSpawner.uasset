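; BP_ProjectileSpawner is an actor that repeatedly fires BP_Projectile instances from its own location.
; From BeginPlay, a self-looping Delay spawns one projectile each Firerate interval.
; Each projectile takes its direction from the ProjectileDirection component's forward vector and its speed from ProjectileSpeed, and calls ProjectileIsLight when ProjIsLight is set.
; The Rotate function is an empty stub.
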(event EventBeginPlay
  ;[0.15 0.15 0.15 0.5] Spawn depending on direction and params
  (Utilities|FlowControl|Delay (Variables|Default|GetFirerate) :!label _label)
  (bind _returnvalue (Game|SpawnActorfromClass "/Game/BlueprintBlocks/Projectile/BP_Projectile.BP_Projectile_C" (Math|Transform|MakeTransform (Transformation|GetActorLocation) "0, 0, 0" "1.000000,1.000000,1.000000") "Undefined" "MultiplyWithRoot" 0 0))
  (Variables|/Game/BlueprintBlocks/Projectile/BP_Projectile.BP_Projectile_C|Setdirection _returnvalue (Math|Vector|GetForwardVector (Variables|Default|GetProjectileDirection)))
  (Variables|/Game/BlueprintBlocks/Projectile/BP_Projectile.BP_Projectile_C|Setspeed _returnvalue (Variables|Default|GetProjectileSpeed))
  (if (Variables|Default|GetProjIsLight)
    (Default|ProjectileIsLight _returnvalue)
    (goto _label)
    (else
      (goto _label))))

(fn ConstructionScript)

(fn Rotate
  (params (NewParam :type Float%20%28double-precision%29)))