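; Base cube for light levels that turns passable inside shadow spheres and becomes solid again when lit.
; Begin and end overlap events count overlapping BP_Shadow_Sphere and BP_Light_Sphere actors.
; These events switch the static mesh's Pawn and GameTraceChannel3 collision responses between Ignore and Block.
; Entering light overrides shadow, but leaving any light restores Ignore whenever shadow remains, without checking for other lights.
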(event Collision|EventActorBeginOverlap
  (params (OtherActor :type Actor%20Object%20Reference))
  (bind _staticmeshcomponent (Variables|Debug|GetStaticMeshComponent))
  (bind _lightcollisions (Variables|Default|GetLightCollisions))
  ;[0.15 0.15 0.15 0.5] Enter Shadow Sphere or Static light
  (Utilities|Casting|CastToBP_Shadow_Sphere OtherActor
    (:then
      (Math|Integer|IncrementInt (Variables|Default|GetShadowCollisions)
        (:%20%20
          (if (== _lightcollisions 0)
            (Collision|SetCollisionResponsetoChannel _staticmeshcomponent "ECC_Pawn" "ECR_Ignore")
            (Collision|SetCollisionResponsetoChannel _staticmeshcomponent "ECC_GameTraceChannel3" "ECR_Ignore")))))
    (:CastFailed
      (Utilities|Casting|CastToBP_Light_Sphere OtherActor)
      (Math|Integer|IncrementInt _lightcollisions
        (:%20%20
          (Collision|SetCollisionResponsetoChannel _staticmeshcomponent "ECC_Pawn" "ECR_Block")
          (Collision|SetCollisionResponsetoChannel _staticmeshcomponent "ECC_GameTraceChannel3" "ECR_Block"))))))

(event Collision|EventActorEndOverlap
  (params (OtherActor :type Actor%20Object%20Reference))
  (bind _staticmeshcomponent (Variables|Debug|GetStaticMeshComponent))
  ;[0.15 0.15 0.15 0.5] Exit Shadow Sphere or Static Light
  (Utilities|Casting|CastToBP_Shadow_Sphere OtherActor
    (:then
      (bind _result (Math|Integer|DecrementInt (Variables|Default|GetShadowCollisions))
        (:%20%20
          (if (== _result 0)
            (Collision|SetCollisionResponsetoChannel _staticmeshcomponent "ECC_Pawn" "ECR_Block")
            (Collision|SetCollisionResponsetoChannel _staticmeshcomponent "ECC_GameTraceChannel3" "ECR_Block")))))
    (:CastFailed
      (Utilities|Casting|CastToBP_Light_Sphere OtherActor)
      (Math|Integer|DecrementInt (Variables|Default|GetLightCollisions)
        (:%20%20
          (if (> (Variables|Default|GetShadowCollisions) 0)
            (Collision|SetCollisionResponsetoChannel _staticmeshcomponent "ECC_Pawn" "ECR_Ignore")
            (Collision|SetCollisionResponsetoChannel _staticmeshcomponent "ECC_GameTraceChannel3" "ECR_Ignore")))))))

(fn ConstructionScript)