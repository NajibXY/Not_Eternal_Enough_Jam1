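; Base cube for the shadow level that toggles whether pawns collide with it, based on overlapping red and blue light spheres.
; Overlap events keep a counter per color and switch the mesh's Pawn channel response.
; Red blocks pawns while no blue overlaps, and any blue entering or the last red leaving sets Ignore.
; Any blue leaving restores Block if red remains, even if other blue still overlaps.
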(event Collision|EventActorBeginOverlap
  (params (OtherActor :type Actor%20Object%20Reference))
  (bind _bluecollisions (Variables|Default|GetBlueCollisions))
  (Utilities|Casting|CastToBP_RedLight_Sphere OtherActor
    (:then
      (Math|Integer|IncrementInt (Variables|Default|GetRedCollisions)
        (:%20%20
          (if (== _bluecollisions 0)
            (Collision|SetCollisionResponsetoChannel (Variables|Debug|GetStaticMeshComponent) "ECC_Pawn" "ECR_Block")))))
    (:CastFailed
      (Utilities|Casting|CastToBP_BlueLight_Sphere OtherActor)
      (Math|Integer|IncrementInt _bluecollisions
        (:%20%20
          (Collision|SetCollisionResponsetoChannel (Variables|Debug|GetStaticMeshComponent) "ECC_Pawn" "ECR_Ignore"))))))

(event Collision|EventActorEndOverlap
  (params (OtherActor :type Actor%20Object%20Reference))
  (bind _redcollisions (Variables|Default|GetRedCollisions))
  (Utilities|Casting|CastToBP_RedLight_Sphere OtherActor
    (:then
      (bind _result (Math|Integer|DecrementInt _redcollisions)
        (:%20%20
          (if (== _result 0)
            (Collision|SetCollisionResponsetoChannel (Variables|Debug|GetStaticMeshComponent) "ECC_Pawn" "ECR_Ignore")))))
    (:CastFailed
      (Utilities|Casting|CastToBP_BlueLight_Sphere OtherActor)
      (Math|Integer|DecrementInt (Variables|Default|GetBlueCollisions)
        (:%20%20
          (if (> _redcollisions 0)
            (Collision|SetCollisionResponsetoChannel (Variables|Debug|GetStaticMeshComponent) "ECC_Pawn" "ECR_Block")))))))

(fn ConstructionScript)