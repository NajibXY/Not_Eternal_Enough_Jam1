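; Base cube for the shadow levels that is made solid while a light sphere overlaps it and passable once the light leaves.
; Overlaps with BP_Light_Sphere set the static mesh to block the Pawn channel and a custom trace channel, and increment a light counter.
; Ending an overlap decrements the counter, restoring Ignore on both channels when it reaches zero, so several lights can overlap the cube at once.
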(event Collision|EventActorBeginOverlap
  (params (OtherActor :type Actor%20Object%20Reference))
  (bind _staticmeshcomponent (Variables|Debug|GetStaticMeshComponent))
  (Utilities|Casting|CastToBP_Light_Sphere OtherActor)
  (Collision|SetCollisionResponsetoChannel _staticmeshcomponent "ECC_Pawn" "ECR_Block")
  (Collision|SetCollisionResponsetoChannel _staticmeshcomponent "ECC_GameTraceChannel3" "ECR_Block")
  (Math|Integer|IncrementInt (Variables|Default|GetLightCollisions)))

(event Collision|EventActorEndOverlap
  (params (OtherActor :type Actor%20Object%20Reference))
  (bind _staticmeshcomponent (Variables|Debug|GetStaticMeshComponent))
  (Utilities|Casting|CastToBP_Light_Sphere OtherActor)
  (bind _result (Math|Integer|DecrementInt (Variables|Default|GetLightCollisions))
    (:%20%20
      (if (== _result 0)
        (Collision|SetCollisionResponsetoChannel _staticmeshcomponent "ECC_Pawn" "ECR_Ignore")
        (Collision|SetCollisionResponsetoChannel _staticmeshcomponent "ECC_GameTraceChannel3" "ECR_Ignore")))))

(fn ConstructionScript)